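; AC_VisionCone is an actor component that computes its owner's field of view and draws it into a render target.
; On BeginPlay it adds a sphere collider sized to the view distance.
; Each tick, a horizontal fan of debug-drawn visibility traces collects hit or max-range points.
; ToCanvasUVTriangles converts those points into triangles, which are drawn onto the cleared canvas render texture as an occlusion-aware vision shape.
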(event `self.ReceiveBeginPlay`
  (bind _returnvalue (`|AddComponentByClass` :`self` (`self.GetOwner`) :`Class` "/Script/Engine.SphereComponent"))
  (bind _output_get (set `self.Collider` _returnvalue))
  (`SphereComponent.SetSphereRadius` _output_get (`self.Distance`) true))

(event `self.ReceiveTick`
  (params (DeltaSeconds :type "Float (single-precision)"))
  (`|ExecutionSequence`
    (:`then_0`
      (`KismetArrayLibrary.Array_Clear` (`self.Hits`))
      (for _index (range (`self.Resolution`))
        (bind _returnvalue (+ (* (`KismetMathLibrary.RotateAngleAxis` (`Actor.GetActorForwardVector` (`self.GetOwner`)) (- (* (`self.Degrees`) _index) (/ (* (`self.Resolution`) (`self.Degrees`)) 2.0)) (0.0 0.0 1.0)) (`self.Distance`)) (`Actor.K2_GetActorLocation` (`self.GetOwner`))))
        (bind (_outhit _returnvalue_2) (`KismetSystemLibrary.LineTraceSingle` :`Start` (`Actor.K2_GetActorLocation` (`self.GetOwner`)) :`End` _returnvalue :`TraceChannel` "TraceTypeQuery1" :`DrawDebugType` "ForOneFrame"))
        (if _returnvalue_2
          (`KismetArrayLibrary.Array_Add` (`self.Hits`) (`.Location` (`GameplayStatics.BreakHitResult` _outhit)))
          (else
            (`KismetArrayLibrary.Array_Add` (`self.Hits`) _returnvalue)))))
    (:`then_1`
      (bind _triangles (`/OpenRTSVision/BFL_RTSVision.ToCanvasUVTriangles` (`self.GetOwner`) (`self.Hits`)))
      (set `self.Triangles` _triangles))
    (:`then_2`
      (`KismetRenderingLibrary.ClearRenderTarget2D` (`self.Canvas Render Texture`))
      (bind (_canvas _size _context) (`KismetRenderingLibrary.BeginDrawCanvasToRenderTarget` (`self.Canvas Render Texture`)))
      (set `self.Context` _context)
      (`Canvas.K2_DrawTriangle` _canvas null (`self.Triangles`))
      (`KismetRenderingLibrary.EndDrawCanvasToRenderTarget` (`self.Context`)))))