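; Actor component that implements a spherical vision strategy, deciding whether its owner can see another actor.
; On BeginPlay it adds a sphere collider to the owner, sized by Distance, and the CanSee check returns whether that collider overlaps the given actor.
; DrawToCanvas renders the same range as a triangle-built circle at the owner's XY world location, with Resolution setting the triangle count.
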(event `self.ReceiveBeginPlay`
  (bind _returnvalue (`|AddComponentByClass` :`self` (`self.GetOwner`) :`Class` "/Script/Engine.SphereComponent"))
  (bind _output_get (set `self.Collider` _returnvalue))
  (`SphereComponent.SetSphereRadius` _output_get (`self.Distance`) true))

(fn `CanSee?`
  (params (Other :type "Actor Object Reference"))
  (returns (NewParam :type Boolean))
  (return (`PrimitiveComponent.IsOverlappingActor` (`self.Collider`) Other)))

(fn `DrawToCanvas`
  (params (Canvas :type "Canvas Object Reference"))
  (bind _returnvalue (`self.GetOwner`))
  (bind _triangles (`/OpenRTSVision/BFL_RTSVision.BuildCircleOfTriangles` _returnvalue (`self.Distance`) (`self.Resolution`) (`KismetMathLibrary.Conv_VectorToVector2D` (`Actor.K2_GetActorLocation` _returnvalue))))
  (`Canvas.K2_DrawTriangle` Canvas null _triangles))