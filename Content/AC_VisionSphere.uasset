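; Actor component that gives its owner a circular vision area, as a collision sphere plus a drawn render-target mask.
; On BeginPlay it adds a sphere component to the owner, sized to the vision Distance.
; Each tick it clears the canvas render texture to black and draws a triangle circle around the owner's XY position.
; BuildCircleOfTriangles generates that shape, with Resolution setting the triangle count.
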(event `self.ReceiveBeginPlay`
  (bind _returnvalue (`|AddComponentByClass` :`self` (`self.GetOwner`) :`Class` "/Script/Engine.SphereComponent"))
  (bind _output_get (set `self.Collider` _returnvalue))
  (`SphereComponent.SetSphereRadius` _output_get (`self.Distance`) true))

(event `self.ReceiveTick`
  (params (DeltaSeconds :type "Float (single-precision)"))
  (bind _returnvalue (`self.GetOwner`))
  (`KismetRenderingLibrary.ClearRenderTarget2D` (`self.Canvas Render Texture`))
  (bind (_canvas _size _context) (`KismetRenderingLibrary.BeginDrawCanvasToRenderTarget` (`self.Canvas Render Texture`)))
  (set `self.Context` _context)
  (bind _triangles (`/OpenRTSVision/BFL_RTSVision.BuildCircleOfTriangles` _returnvalue (`self.Distance`) (`self.Resolution`) (`KismetMathLibrary.Conv_VectorToVector2D` (`Actor.K2_GetActorLocation` _returnvalue))))
  (`Canvas.K2_DrawTriangle` _canvas null _triangles)
  (`KismetRenderingLibrary.EndDrawCanvasToRenderTarget` (`self.Context`)))