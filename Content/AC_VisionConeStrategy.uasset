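; Actor component vision strategy that gives its owner a cone of sight and draws it onto a canvas.
; On BeginPlay it adds a sphere collider sized to the view distance.
; CanSee tests only whether a target's relative yaw lies within the cone, ignoring distance and occlusion.
; DrawToCanvas fans Visibility traces across the cone and converts hit or max-range points to triangles, so obstacles clip the drawn shape.
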(event `self.ReceiveBeginPlay`
  (bind _returnvalue (`|AddComponentByClass` :`self` (`self.GetOwner`) :`Class` "/Script/Engine.SphereComponent"))
  (bind _output_get (set `self.Collider` _returnvalue))
  (`SphereComponent.SetSphereRadius` _output_get (`self.Distance`) true))

(fn `CanSee?`
  (params (Other :type "Actor Object Reference"))
  (returns (NewParam :type Boolean))
  (bind (_returnvalue_roll _returnvalue_pitch _returnvalue_yaw) (`KismetMathLibrary.BreakRotator` (`KismetMathLibrary.FindRelativeLookAtRotation` (`Actor.GetTransform` (`self.GetOwner`)) (`Actor.K2_GetActorLocation` Other))))
  (return (<= (`KismetMathLibrary.Abs` _returnvalue_yaw) (/ (* (`self.Degrees`) (`self.Resolution`)) 2.0))))

(fn `DrawToCanvas`
  (params (Canvas :type "Canvas Object Reference"))
  (`|ExecutionSequence`
    (:`then_0`
      (`KismetArrayLibrary.Array_Clear` (`self.Hits`))
      (for _index (range (`self.Resolution`))
        (bind _returnvalue (+ (* (`KismetMathLibrary.RotateAngleAxis` (`Actor.GetActorForwardVector` (`self.GetOwner`)) (- (* (`self.Degrees`) _index) (/ (* (`self.Resolution`) (`self.Degrees`)) 2.0)) (0.0 0.0 1.0)) (`self.Distance`)) (`Actor.K2_GetActorLocation` (`self.GetOwner`))))
        (bind (_outhit _returnvalue_2) (`KismetSystemLibrary.LineTraceSingle` :`Start` (`Actor.K2_GetActorLocation` (`self.GetOwner`)) :`End` _returnvalue :`TraceChannel` "TraceTypeQuery1" :`DrawDebugType` "ForOneFrame"))
        (if _returnvalue_2
          (`KismetArrayLibrary.Array_Add` (`self.Hits`) (`.Location` (`GameplayStatics.BreakHitResult` _outhit)))
          (else
            (`KismetArrayLibrary.Array_Add` (`self.Hits`) _returnvalue)))))
    (:`then_1`
      (bind _triangles (`/OpenRTSVision/BFL_RTSVision.ToCanvasUVTriangles` (`self.GetOwner`) (`self.Hits`)))
      (set `self.Triangles` _triangles))
    (:`then_2`
      (`Canvas.K2_DrawTriangle` Canvas null (`self.Triangles`)))))