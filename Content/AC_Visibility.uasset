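; AC_Visibility is an actor component that hides its owner unless an overlapping actor can see it.
; On BeginPlay it adds a box collider to the owner, with its extent set from Size.
; Every tick it hides the owner, then asks each overlapping actor's AC_VisionManager whether it can see the owner.
; Any positive CanSee result makes the owner visible again for that frame.
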(event `self.ReceiveBeginPlay`
  (bind _returnvalue (`|AddComponentByClass` :`self` (`self.GetOwner`) :`Class` "/Script/Engine.BoxComponent"))
  (bind _output_get (set `self.Collider` _returnvalue))
  (`BoxComponent.SetBoxExtent` _output_get (`KismetMathLibrary.Conv_DoubleToVector` (`self.Size`)) true))

(event `self.ReceiveTick`
  (params (DeltaSeconds :type "Float (single-precision)"))
  (bind _overlappingactors (`PrimitiveComponent.GetOverlappingActors` (`self.Collider`) null))
  (`Actor.SetActorHiddenInGame` (`self.GetOwner`) true)
  (if (not (`KismetArrayLibrary.Array_IsEmpty` _overlappingactors))
    (for _array_element _overlappingactors
      (bind _returnvalue (`Actor.GetComponentByClass` _array_element "/OpenRTSVision/AC_VisionManager.AC_VisionManager_C"))
      (`/Engine/EditorBlueprintResources/StandardMacros.IsValid` _returnvalue
        (:`Is Valid`
          (bind _cansee (`/OpenRTSVision/AC_VisionManager.CanSee?` _returnvalue (`self.GetOwner`)))
          (if _cansee
            (`Actor.SetActorHiddenInGame` (`self.GetOwner`) false)))))))