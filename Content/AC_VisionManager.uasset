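; AC_VisionManager is an actor component that combines its owner's vision strategies into one rendered vision mask and one visibility query.
; On BeginPlay it gathers every AC_VisionStrategyBase component on the owner.
; Each tick it clears a canvas render target to black and lets each strategy draw onto it.
; CanSee returns true as soon as any strategy reports seeing the other object.
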(event `self.ReceiveBeginPlay`
  (set `self.Vision Strategies` (`Actor.K2_GetComponentsByClass` (`self.GetOwner`) "/OpenRTSVision/AC_VisionStrategyBase.AC_VisionStrategyBase_C")))

(event `self.ReceiveTick`
  (params (DeltaSeconds :type "Float (single-precision)"))
  (`KismetRenderingLibrary.ClearRenderTarget2D` (`self.Canvas Render Target`))
  (bind (_canvas _size _context) (`KismetRenderingLibrary.BeginDrawCanvasToRenderTarget` (`self.Canvas Render Target`)))
  (for _array_element (`self.Vision Strategies`)
    (`/OpenRTSVision/AC_VisionStrategyBase.DrawToCanvas` _array_element _canvas))
  (`KismetRenderingLibrary.EndDrawCanvasToRenderTarget` _context))

(fn `CanSee?`
  (params (Other :type "Actor Object Reference"))
  (returns (CanSee :type Boolean))
  (for _array_element (`self.Vision Strategies`)
    (bind _newparam (`/OpenRTSVision/AC_VisionStrategyBase.CanSee?` _array_element Other))
    (if _newparam
      (return true)))
  (return false))